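; Scene capture camera that captures the character into a render target for snow effects, only while over snow-tagged actors.
; BeginPlay sizes the orthographic capture from MPC_RenderTargetData, creates an M_Capture_Character material instance and clears the target.
; Each tick draws that material to the target, then sphere-traces behind the camera for the "snow" tag.
; The result toggles the capture's max view distance between unlimited and near-zero, effectively gating what it records.
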(event EventBeginPlay
  ;[1 1 1 1 90] Create material to draw
  (bind _returnvalue (Rendering|Material|GetScalarParameterValue "/Game/Snow_FX/Materials/MaterialParameterCollection/MPC_RenderTargetData.MPC_RenderTargetData" "Capture width (Character)" :!class /Script/Engine.KismetMaterialLibrary))
  (Variables|/Script/Engine.SceneCaptureComponent2D|SetOrthoWidth (Variables|Default|GetSceneCaptureComponent2D) _returnvalue)
  (Variables|/Script/Engine.SceneCaptureComponent|SetMaxViewDistanceOverride (Variables|Default|GetSceneCaptureComponent2D) 1.0)
  (bind _returnvalue_2 (Rendering|Material|CreateDynamicMaterialInstance "/Game/Snow_FX/Materials/RenderTarget_Materials/M_Capture_Character.M_Capture_Character" "None" "None" :!class /Script/Engine.KismetMaterialLibrary))
  (Variables|Default|SetMat _returnvalue_2)
  (Rendering|ClearRenderTarget2D (Variables|Default|GetRenderTarget)))

(event EventTick
  (params (DeltaSeconds :type Float%20%28single-precision%29))
  (bind _defaultsceneroot (Variables|Default|GetDefaultSceneRoot))
  (bind _scenecapturecomponent2d (Variables|Default|GetSceneCaptureComponent2D))
  (bind _returnvalue (Transformation|GetWorldLocation _defaultsceneroot))
  ;[0 0.1939 1 1 90] Check Snow layer to Capture
  (Rendering|DrawMaterialtoRenderTarget (Variables|Default|GetRenderTarget) (Variables|Default|GetMat))
  (bind (_outhit _returnvalue_2) (Collision|SphereTraceByChannel _returnvalue (+ _returnvalue (* (Math|Vector|GetForwardVector (Variables|Default|GetSceneCaptureComponent2D)) -10)) 5.0 "TraceTypeQuery1" true 0 "None"))
  (if _returnvalue_2
    (Variables|Default|SetSnow (Actor|ActorHasTag (.HitActor (Collision|BreakHitResult _outhit)) "snow"))
    (else
      (Variables|Default|SetSnow false)))
  (if (Variables|Default|GetSnow)
    (Variables|/Script/Engine.SceneCaptureComponent|SetMaxViewDistanceOverride _scenecapturecomponent2d -1.0)
    (else
      (Variables|/Script/Engine.SceneCaptureComponent|SetMaxViewDistanceOverride _scenecapturecomponent2d 1.0))))

(fn ConstructionScript)