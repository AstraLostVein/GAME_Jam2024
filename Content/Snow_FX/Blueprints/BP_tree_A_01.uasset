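; Snowy tree actor whose individual leaf collision components react to overlaps with material-driven movement and falling snow.
; Each overlap calls HitLeaf, which passes leaf ID, hit time and move amount to the tree mesh's materials as scalar parameters.
; A DoOnce per leaf spawns the Fall_Snow_Emitter_System Niagara effect at that leaf on first overlap only, except Leaf_48, which spawns none.
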(event OnComponentBeginOverlap(Leaf_01)
  (params (OverlappedComponent :type Primitive%20Component%20Object%20Reference) (OtherActor :type Actor%20Object%20Reference) (OtherComp :type Primitive%20Component%20Object%20Reference) (OtherBodyIndex :type Integer) (bFromSweep :type Boolean) (SweepResult :type Hit%20Result%20Structure%20%28by%20ref%29))
  ;[0.09468 0 1 1 90] Leafs collision setup
  (CallFunction|Leaf 1 "leaf_01" 2e+01)
  (Utilities|FlowControl|DoOnce false
    (:Completed
      (CallFunction|SpawnNiagara (Transformation|GetWorldTransform (Variables|Default|GetLeaf_01))))))

(event OnComponentBeginOverlap(Leaf_02)
  (params (OverlappedComponent :type Primitive%20Component%20Object%20Reference) (OtherActor :type Actor%20Object%20Reference) (OtherComp :type Primitive%20Component%20Object%20Reference) (OtherBodyIndex :type Integer) (bFromSweep :type Boolean) (SweepResult :type Hit%20Result%20Structure%20%28by%20ref%29))
  ;[0.09468 0 1 1 90] Leafs collision setup
  (CallFunction|Leaf 2 "leaf_02" 2e+01)
  (Utilities|FlowControl|DoOnce false
    (:Completed
      (CallFunction|SpawnNiagara (Transformation|GetWorldTransform (Variables|Default|GetLeaf_02))))))

(event OnComponentBeginOverlap(Leaf_11)
  (params (OverlappedComponent :type Primitive%20Component%20Object%20Reference) (OtherActor :type Actor%20Object%20Reference) (OtherComp :type Primitive%20Component%20Object%20Reference) (OtherBodyIndex :type Integer) (bFromSweep :type Boolean) (SweepResult :type Hit%20Result%20Structure%20%28by%20ref%29))
  ;[0.09468 0 1 1 90] Leafs collision setup
  (CallFunction|Leaf 11 "leaf_11" 4e+01)
  (Utilities|FlowControl|DoOnce false
    (:Completed
      (CallFunction|SpawnNiagara (Transformation|GetWorldTransform (Variables|Default|GetLeaf_11))))))

(event OnComponentBeginOverlap(Leaf_12)
  (params (OverlappedComponent :type Primitive%20Component%20Object%20Reference) (OtherActor :type Actor%20Object%20Reference) (OtherComp :type Primitive%20Component%20Object%20Reference) (OtherBodyIndex :type Integer) (bFromSweep :type Boolean) (SweepResult :type Hit%20Result%20Structure%20%28by%20ref%29))
  ;[0.09468 0 1 1 90] Leafs collision setup
  (CallFunction|Leaf 12 "leaf_12" 4e+01)
  (Utilities|FlowControl|DoOnce false
    (:Completed
      (CallFunction|SpawnNiagara (Transformation|GetWorldTransform (Variables|Default|GetLeaf_12))))))

(event OnComponentBeginOverlap(Leaf_13)
  (params (OverlappedComponent :type Primitive%20Component%20Object%20Reference) (OtherActor :type Actor%20Object%20Reference) (OtherComp :type Primitive%20Component%20Object%20Reference) (OtherBodyIndex :type Integer) (bFromSweep :type Boolean) (SweepResult :type Hit%20Result%20Structure%20%28by%20ref%29))
  ;[0.09468 0 1 1 90] Leafs collision setup
  (CallFunction|Leaf 13 "leaf_13" 4e+01)
  (Utilities|FlowControl|DoOnce false
    (:Completed
      (CallFunction|SpawnNiagara (Transformation|GetWorldTransform (Variables|Default|GetLeaf_13))))))

(event OnComponentBeginOverlap(Leaf_14)
  (params (OverlappedComponent :type Primitive%20Component%20Object%20Reference) (OtherActor :type Actor%20Object%20Reference) (OtherComp :type Primitive%20Component%20Object%20Reference) (OtherBodyIndex :type Integer) (bFromSweep :type Boolean) (SweepResult :type Hit%20Result%20Structure%20%28by%20ref%29))
  ;[0.09468 0 1 1 90] Leafs collision setup
  (CallFunction|Leaf 14 "leaf_14" 4e+01)
  (Utilities|FlowControl|DoOnce false
    (:Completed
      (CallFunction|SpawnNiagara (Transformation|GetWorldTransform (Variables|Default|GetLeaf_14))))))

(event OnComponentBeginOverlap(Leaf_15)
  (params (OverlappedComponent :type Primitive%20Component%20Object%20Reference) (OtherActor :type Actor%20Object%20Reference) (OtherComp :type Primitive%20Component%20Object%20Reference) (OtherBodyIndex :type Integer) (bFromSweep :type Boolean) (SweepResult :type Hit%20Result%20Structure%20%28by%20ref%29))
  ;[0.09468 0 1 1 90] Leafs collision setup
  (CallFunction|Leaf 15 "leaf_15" 4e+01)
  (Utilities|FlowControl|DoOnce false
    (:Completed
      (CallFunction|SpawnNiagara (Transformation|GetWorldTransform (Variables|Default|GetLeaf_15))))))

(event OnComponentBeginOverlap(Leaf_16)
  (params (OverlappedComponent :type Primitive%20Component%20Object%20Reference) (OtherActor :type Actor%20Object%20Reference) (OtherComp :type Primitive%20Component%20Object%20Reference) (OtherBodyIndex :type Integer) (bFromSweep :type Boolean) (SweepResult :type Hit%20Result%20Structure%20%28by%20ref%29))
  ;[0.09468 0 1 1 90] Leafs collision setup
  (CallFunction|Leaf 16 "leaf_16" 4e+01)
  (Utilities|FlowControl|DoOnce false
    (:Completed
      (CallFunction|SpawnNiagara (Transformation|GetWorldTransform (Variables|Default|GetLeaf_16))))))

(event OnComponentBeginOverlap(Leaf_17)
  (params (OverlappedComponent :type Primitive%20Component%20Object%20Reference) (OtherActor :type Actor%20Object%20Reference) (OtherComp :type Primitive%20Component%20Object%20Reference) (OtherBodyIndex :type Integer) (bFromSweep :type Boolean) (SweepResult :type Hit%20Result%20Structure%20%28by%20ref%29))
  ;[0.09468 0 1 1 90] Leafs collision setup
  (CallFunction|Leaf 17 "leaf_17" 4e+01)
  (Utilities|FlowControl|DoOnce false
    (:Completed
      (CallFunction|SpawnNiagara (Transformation|GetWorldTransform (Variables|Default|GetLeaf_17))))))

(event OnComponentBeginOverlap(Leaf_18)
  (params (OverlappedComponent :type Primitive%20Component%20Object%20Reference) (OtherActor :type Actor%20Object%20Reference) (OtherComp :type Primitive%20Component%20Object%20Reference) (OtherBodyIndex :type Integer) (bFromSweep :type Boolean) (SweepResult :type Hit%20Result%20Structure%20%28by%20ref%29))
  ;[0.09468 0 1 1 90] Leafs collision setup
  (CallFunction|Leaf 18 "leaf_18" 4e+01)
  (Utilities|FlowControl|DoOnce false
    (:Completed
      (CallFunction|SpawnNiagara (Transformation|GetWorldTransform (Variables|Default|GetLeaf_18))))))

(event OnComponentBeginOverlap(Leaf_19)
  (params (OverlappedComponent :type Primitive%20Component%20Object%20Reference) (OtherActor :type Actor%20Object%20Reference) (OtherComp :type Primitive%20Component%20Object%20Reference) (OtherBodyIndex :type Integer) (bFromSweep :type Boolean) (SweepResult :type Hit%20Result%20Structure%20%28by%20ref%29))
  ;[0.09468 0 1 1 90] Leafs collision setup
  (CallFunction|Leaf 19 "leaf_19" 4e+01)
  (Utilities|FlowControl|DoOnce false
    (:Completed
      (CallFunction|SpawnNiagara (Transformation|GetWorldTransform (Variables|Default|GetLeaf_19))))))

(event OnComponentBeginOverlap(Leaf_20)
  (params (OverlappedComponent :type Primitive%20Component%20Object%20Reference) (OtherActor :type Actor%20Object%20Reference) (OtherComp :type Primitive%20Component%20Object%20Reference) (OtherBodyIndex :type Integer) (bFromSweep :type Boolean) (SweepResult :type Hit%20Result%20Structure%20%28by%20ref%29))
  ;[0.09468 0 1 1 90] Leafs collision setup
  (CallFunction|Leaf 20 "leaf_20" 4e+01)
  (Utilities|FlowControl|DoOnce false
    (:Completed
      (CallFunction|SpawnNiagara (Transformation|GetWorldTransform (Variables|Default|GetLeaf_20))))))

(event OnComponentBeginOverlap(Leaf_03)
  (params (OverlappedComponent :type Primitive%20Component%20Object%20Reference) (OtherActor :type Actor%20Object%20Reference) (OtherComp :type Primitive%20Component%20Object%20Reference) (OtherBodyIndex :type Integer) (bFromSweep :type Boolean) (SweepResult :type Hit%20Result%20Structure%20%28by%20ref%29))
  ;[0.09468 0 1 1 90] Leafs collision setup
  (CallFunction|Leaf 3 "leaf_03" 4e+01)
  (Utilities|FlowControl|DoOnce false
    (:Completed
      (CallFunction|SpawnNiagara (Transformation|GetWorldTransform (Variables|Default|GetLeaf_03))))))

(event OnComponentBeginOverlap(Leaf_21)
  (params (OverlappedComponent :type Primitive%20Component%20Object%20Reference) (OtherActor :type Actor%20Object%20Reference) (OtherComp :type Primitive%20Component%20Object%20Reference) (OtherBodyIndex :type Integer) (bFromSweep :type Boolean) (SweepResult :type Hit%20Result%20Structure%20%28by%20ref%29))
  ;[0.09468 0 1 1 90] Leafs collision setup
  (CallFunction|Leaf 21 "leaf_21" 4e+01)
  (Utilities|FlowControl|DoOnce false
    (:Completed
      (CallFunction|SpawnNiagara (Transformation|GetWorldTransform (Variables|Default|GetLeaf_21))))))

(event OnComponentBeginOverlap(Leaf_22)
  (params (OverlappedComponent :type Primitive%20Component%20Object%20Reference) (OtherActor :type Actor%20Object%20Reference) (OtherComp :type Primitive%20Component%20Object%20Reference) (OtherBodyIndex :type Integer) (bFromSweep :type Boolean) (SweepResult :type Hit%20Result%20Structure%20%28by%20ref%29))
  ;[0.09468 0 1 1 90] Leafs collision setup
  (CallFunction|Leaf 22 "leaf_22" 4e+01)
  (Utilities|FlowControl|DoOnce false
    (:Completed
      (CallFunction|SpawnNiagara (Transformation|GetWorldTransform (Variables|Default|GetLeaf_22))))))

(event OnComponentBeginOverlap(Leaf_23)
  (params (OverlappedComponent :type Primitive%20Component%20Object%20Reference) (OtherActor :type Actor%20Object%20Reference) (OtherComp :type Primitive%20Component%20Object%20Reference) (OtherBodyIndex :type Integer) (bFromSweep :type Boolean) (SweepResult :type Hit%20Result%20Structure%20%28by%20ref%29))
  ;[0.09468 0 1 1 90] Leafs collision setup
  (CallFunction|Leaf 23 "leaf_23" 4e+01)
  (Utilities|FlowControl|DoOnce false
    (:Completed
      (CallFunction|SpawnNiagara (Transformation|GetWorldTransform (Variables|Default|GetLeaf_23))))))

(event OnComponentBeginOverlap(Leaf_24)
  (params (OverlappedComponent :type Primitive%20Component%20Object%20Reference) (OtherActor :type Actor%20Object%20Reference) (OtherComp :type Primitive%20Component%20Object%20Reference) (OtherBodyIndex :type Integer) (bFromSweep :type Boolean) (SweepResult :type Hit%20Result%20Structure%20%28by%20ref%29))
  ;[0.09468 0 1 1 90] Leafs collision setup
  (CallFunction|Leaf 24 "leaf_24" 4e+01)
  (Utilities|FlowControl|DoOnce false
    (:Completed
      (CallFunction|SpawnNiagara (Transformation|GetWorldTransform (Variables|Default|GetLeaf_24))))))

(event OnComponentBeginOverlap(Leaf_25)
  (params (OverlappedComponent :type Primitive%20Component%20Object%20Reference) (OtherActor :type Actor%20Object%20Reference) (OtherComp :type Primitive%20Component%20Object%20Reference) (OtherBodyIndex :type Integer) (bFromSweep :type Boolean) (SweepResult :type Hit%20Result%20Structure%20%28by%20ref%29))
  ;[0.09468 0 1 1 90] Leafs collision setup
  (CallFunction|Leaf 25 "leaf_25" 4e+01)
  (Utilities|FlowControl|DoOnce false
    (:Completed
      (CallFunction|SpawnNiagara (Transformation|GetWorldTransform (Variables|Default|GetLeaf_25))))))

(event OnComponentBeginOverlap(Leaf_26)
  (params (OverlappedComponent :type Primitive%20Component%20Object%20Reference) (OtherActor :type Actor%20Object%20Reference) (OtherComp :type Primitive%20Component%20Object%20Reference) (OtherBodyIndex :type Integer) (bFromSweep :type Boolean) (SweepResult :type Hit%20Result%20Structure%20%28by%20ref%29))
  ;[0.09468 0 1 1 90] Leafs collision setup
  (CallFunction|Leaf 26 "leaf_26" 4e+01)
  (Utilities|FlowControl|DoOnce false
    (:Completed
      (CallFunction|SpawnNiagara (Transformation|GetWorldTransform (Variables|Default|GetLeaf_26))))))

(event OnComponentBeginOverlap(Leaf_27)
  (params (OverlappedComponent :type Primitive%20Component%20Object%20Reference) (OtherActor :type Actor%20Object%20Reference) (OtherComp :type Primitive%20Component%20Object%20Reference) (OtherBodyIndex :type Integer) (bFromSweep :type Boolean) (SweepResult :type Hit%20Result%20Structure%20%28by%20ref%29))
  ;[0.09468 0 1 1 90] Leafs collision setup
  (CallFunction|Leaf 27 "leaf_27" 4e+01)
  (Utilities|FlowControl|DoOnce false
    (:Completed
      (CallFunction|SpawnNiagara (Transformation|GetWorldTransform (Variables|Default|GetLeaf_27))))))

(event OnComponentBeginOverlap(Leaf_28)
  (params (OverlappedComponent :type Primitive%20Component%20Object%20Reference) (OtherActor :type Actor%20Object%20Reference) (OtherComp :type Primitive%20Component%20Object%20Reference) (OtherBodyIndex :type Integer) (bFromSweep :type Boolean) (SweepResult :type Hit%20Result%20Structure%20%28by%20ref%29))
  ;[0.09468 0 1 1 90] Leafs collision setup
  (CallFunction|Leaf 28 "leaf_28" 4e+01)
  (Utilities|FlowControl|DoOnce false
    (:Completed
      (CallFunction|SpawnNiagara (Transformation|GetWorldTransform (Variables|Default|GetLeaf_28))))))

(event OnComponentBeginOverlap(Leaf_29)
  (params (OverlappedComponent :type Primitive%20Component%20Object%20Reference) (OtherActor :type Actor%20Object%20Reference) (OtherComp :type Primitive%20Component%20Object%20Reference) (OtherBodyIndex :type Integer) (bFromSweep :type Boolean) (SweepResult :type Hit%20Result%20Structure%20%28by%20ref%29))
  ;[0.09468 0 1 1 90] Leafs collision setup
  (CallFunction|Leaf 29 "leaf_29" 4e+01)
  (Utilities|FlowControl|DoOnce false
    (:Completed
      (CallFunction|SpawnNiagara (Transformation|GetWorldTransform (Variables|Default|GetLeaf_29))))))

(event OnComponentBeginOverlap(Leaf_30)
  (params (OverlappedComponent :type Primitive%20Component%20Object%20Reference) (OtherActor :type Actor%20Object%20Reference) (OtherComp :type Primitive%20Component%20Object%20Reference) (OtherBodyIndex :type Integer) (bFromSweep :type Boolean) (SweepResult :type Hit%20Result%20Structure%20%28by%20ref%29))
  ;[0.09468 0 1 1 90] Leafs collision setup
  (CallFunction|Leaf 30 "leaf_30" 4e+01)
  (Utilities|FlowControl|DoOnce false
    (:Completed
      (CallFunction|SpawnNiagara (Transformation|GetWorldTransform (Variables|Default|GetLeaf_30))))))

(event OnComponentBeginOverlap(Leaf_04)
  (params (OverlappedComponent :type Primitive%20Component%20Object%20Reference) (OtherActor :type Actor%20Object%20Reference) (OtherComp :type Primitive%20Component%20Object%20Reference) (OtherBodyIndex :type Integer) (bFromSweep :type Boolean) (SweepResult :type Hit%20Result%20Structure%20%28by%20ref%29))
  ;[0.09468 0 1 1 90] Leafs collision setup
  (CallFunction|Leaf 4 "leaf_04" 4e+01)
  (Utilities|FlowControl|DoOnce false
    (:Completed
      (CallFunction|SpawnNiagara (Transformation|GetWorldTransform (Variables|Default|GetLeaf_04))))))

(event OnComponentBeginOverlap(Leaf_31)
  (params (OverlappedComponent :type Primitive%20Component%20Object%20Reference) (OtherActor :type Actor%20Object%20Reference) (OtherComp :type Primitive%20Component%20Object%20Reference) (OtherBodyIndex :type Integer) (bFromSweep :type Boolean) (SweepResult :type Hit%20Result%20Structure%20%28by%20ref%29))
  ;[0.09468 0 1 1 90] Leafs collision setup
  (CallFunction|Leaf 31 "leaf_31" 4e+01)
  (Utilities|FlowControl|DoOnce false
    (:Completed
      (CallFunction|SpawnNiagara (Transformation|GetWorldTransform (Variables|Default|GetLeaf_31))))))

(event OnComponentBeginOverlap(Leaf_32)
  (params (OverlappedComponent :type Primitive%20Component%20Object%20Reference) (OtherActor :type Actor%20Object%20Reference) (OtherComp :type Primitive%20Component%20Object%20Reference) (OtherBodyIndex :type Integer) (bFromSweep :type Boolean) (SweepResult :type Hit%20Result%20Structure%20%28by%20ref%29))
  ;[0.09468 0 1 1 90] Leafs collision setup
  (CallFunction|Leaf 32 "leaf_32" 4e+01)
  (Utilities|FlowControl|DoOnce false
    (:Completed
      (CallFunction|SpawnNiagara (Transformation|GetWorldTransform (Variables|Default|GetLeaf_32))))))

(event OnComponentBeginOverlap(Leaf_33)
  (params (OverlappedComponent :type Primitive%20Component%20Object%20Reference) (OtherActor :type Actor%20Object%20Reference) (OtherComp :type Primitive%20Component%20Object%20Reference) (OtherBodyIndex :type Integer) (bFromSweep :type Boolean) (SweepResult :type Hit%20Result%20Structure%20%28by%20ref%29))
  ;[0.09468 0 1 1 90] Leafs collision setup
  (CallFunction|Leaf 33 "leaf_33" 4e+01)
  (Utilities|FlowControl|DoOnce false
    (:Completed
      (CallFunction|SpawnNiagara (Transformation|GetWorldTransform (Variables|Default|GetLeaf_33))))))

(event OnComponentBeginOverlap(Leaf_34)
  (params (OverlappedComponent :type Primitive%20Component%20Object%20Reference) (OtherActor :type Actor%20Object%20Reference) (OtherComp :type Primitive%20Component%20Object%20Reference) (OtherBodyIndex :type Integer) (bFromSweep :type Boolean) (SweepResult :type Hit%20Result%20Structure%20%28by%20ref%29))
  ;[0.09468 0 1 1 90] Leafs collision setup
  (CallFunction|Leaf 34 "leaf_34" 4e+01)
  (Utilities|FlowControl|DoOnce false
    (:Completed
      (CallFunction|SpawnNiagara (Transformation|GetWorldTransform (Variables|Default|GetLeaf_34))))))

(event OnComponentBeginOverlap(Leaf_35)
  (params (OverlappedComponent :type Primitive%20Component%20Object%20Reference) (OtherActor :type Actor%20Object%20Reference) (OtherComp :type Primitive%20Component%20Object%20Reference) (OtherBodyIndex :type Integer) (bFromSweep :type Boolean) (SweepResult :type Hit%20Result%20Structure%20%28by%20ref%29))
  ;[0.09468 0 1 1 90] Leafs collision setup
  (CallFunction|Leaf 35 "leaf_35" 4e+01)
  (Utilities|FlowControl|DoOnce false
    (:Completed
      (CallFunction|SpawnNiagara (Transformation|GetWorldTransform (Variables|Default|GetLeaf_35))))))

(event OnComponentBeginOverlap(Leaf_36)
  (params (OverlappedComponent :type Primitive%20Component%20Object%20Reference) (OtherActor :type Actor%20Object%20Reference) (OtherComp :type Primitive%20Component%20Object%20Reference) (OtherBodyIndex :type Integer) (bFromSweep :type Boolean) (SweepResult :type Hit%20Result%20Structure%20%28by%20ref%29))
  ;[0.09468 0 1 1 90] Leafs collision setup
  (CallFunction|Leaf 36 "leaf_36" 4e+01)
  (Utilities|FlowControl|DoOnce false
    (:Completed
      (CallFunction|SpawnNiagara (Transformation|GetWorldTransform (Variables|Default|GetLeaf_36))))))

(event OnComponentBeginOverlap(Leaf_37)
  (params (OverlappedComponent :type Primitive%20Component%20Object%20Reference) (OtherActor :type Actor%20Object%20Reference) (OtherComp :type Primitive%20Component%20Object%20Reference) (OtherBodyIndex :type Integer) (bFromSweep :type Boolean) (SweepResult :type Hit%20Result%20Structure%20%28by%20ref%29))
  ;[0.09468 0 1 1 90] Leafs collision setup
  (CallFunction|Leaf 37 "leaf_37" 4e+01)
  (Utilities|FlowControl|DoOnce false
    (:Completed
      (CallFunction|SpawnNiagara (Transformation|GetWorldTransform (Variables|Default|GetLeaf_37))))))

(event OnComponentBeginOverlap(Leaf_38)
  (params (OverlappedComponent :type Primitive%20Component%20Object%20Reference) (OtherActor :type Actor%20Object%20Reference) (OtherComp :type Primitive%20Component%20Object%20Reference) (OtherBodyIndex :type Integer) (bFromSweep :type Boolean) (SweepResult :type Hit%20Result%20Structure%20%28by%20ref%29))
  ;[0.09468 0 1 1 90] Leafs collision setup
  (CallFunction|Leaf 38 "leaf_38" 4e+01)
  (Utilities|FlowControl|DoOnce false
    (:Completed
      (CallFunction|SpawnNiagara (Transformation|GetWorldTransform (Variables|Default|GetLeaf_38))))))

(event OnComponentBeginOverlap(Leaf_39)
  (params (OverlappedComponent :type Primitive%20Component%20Object%20Reference) (OtherActor :type Actor%20Object%20Reference) (OtherComp :type Primitive%20Component%20Object%20Reference) (OtherBodyIndex :type Integer) (bFromSweep :type Boolean) (SweepResult :type Hit%20Result%20Structure%20%28by%20ref%29))
  ;[0.09468 0 1 1 90] Leafs collision setup
  (CallFunction|Leaf 39 "leaf_39" 4e+01)
  (Utilities|FlowControl|DoOnce false
    (:Completed
      (CallFunction|SpawnNiagara (Transformation|GetWorldTransform (Variables|Default|GetLeaf_39))))))

(event OnComponentBeginOverlap(Leaf_40)
  (params (OverlappedComponent :type Primitive%20Component%20Object%20Reference) (OtherActor :type Actor%20Object%20Reference) (OtherComp :type Primitive%20Component%20Object%20Reference) (OtherBodyIndex :type Integer) (bFromSweep :type Boolean) (SweepResult :type Hit%20Result%20Structure%20%28by%20ref%29))
  ;[0.09468 0 1 1 90] Leafs collision setup
  (CallFunction|Leaf 40 "leaf_40" 4e+01)
  (Utilities|FlowControl|DoOnce false
    (:Completed
      (CallFunction|SpawnNiagara (Transformation|GetWorldTransform (Variables|Default|GetLeaf_40))))))

(event OnComponentBeginOverlap(Leaf_05)
  (params (OverlappedComponent :type Primitive%20Component%20Object%20Reference) (OtherActor :type Actor%20Object%20Reference) (OtherComp :type Primitive%20Component%20Object%20Reference) (OtherBodyIndex :type Integer) (bFromSweep :type Boolean) (SweepResult :type Hit%20Result%20Structure%20%28by%20ref%29))
  ;[0.09468 0 1 1 90] Leafs collision setup
  (CallFunction|Leaf 5 "leaf_05" 4e+01)
  (Utilities|FlowControl|DoOnce false
    (:Completed
      (CallFunction|SpawnNiagara (Transformation|GetWorldTransform (Variables|Default|GetLeaf_05))))))

(event OnComponentBeginOverlap(Leaf_41)
  (params (OverlappedComponent :type Primitive%20Component%20Object%20Reference) (OtherActor :type Actor%20Object%20Reference) (OtherComp :type Primitive%20Component%20Object%20Reference) (OtherBodyIndex :type Integer) (bFromSweep :type Boolean) (SweepResult :type Hit%20Result%20Structure%20%28by%20ref%29))
  ;[0.09468 0 1 1 90] Leafs collision setup
  (CallFunction|Leaf 41 "leaf_41" 4e+01)
  (Utilities|FlowControl|DoOnce false
    (:Completed
      (CallFunction|SpawnNiagara (Transformation|GetWorldTransform (Variables|Default|GetLeaf_41))))))

(event OnComponentBeginOverlap(Leaf_42)
  (params (OverlappedComponent :type Primitive%20Component%20Object%20Reference) (OtherActor :type Actor%20Object%20Reference) (OtherComp :type Primitive%20Component%20Object%20Reference) (OtherBodyIndex :type Integer) (bFromSweep :type Boolean) (SweepResult :type Hit%20Result%20Structure%20%28by%20ref%29))
  ;[0.09468 0 1 1 90] Leafs collision setup
  (CallFunction|Leaf 42 "leaf_42" 4e+01)
  (Utilities|FlowControl|DoOnce false
    (:Completed
      (CallFunction|SpawnNiagara (Transformation|GetWorldTransform (Variables|Default|GetLeaf_42))))))

(event OnComponentBeginOverlap(Leaf_43)
  (params (OverlappedComponent :type Primitive%20Component%20Object%20Reference) (OtherActor :type Actor%20Object%20Reference) (OtherComp :type Primitive%20Component%20Object%20Reference) (OtherBodyIndex :type Integer) (bFromSweep :type Boolean) (SweepResult :type Hit%20Result%20Structure%20%28by%20ref%29))
  ;[0.09468 0 1 1 90] Leafs collision setup
  (CallFunction|Leaf 43 "leaf_43" 4e+01)
  (Utilities|FlowControl|DoOnce false
    (:Completed
      (CallFunction|SpawnNiagara (Transformation|GetWorldTransform (Variables|Default|GetLeaf_43))))))

(event OnComponentBeginOverlap(Leaf_44)
  (params (OverlappedComponent :type Primitive%20Component%20Object%20Reference) (OtherActor :type Actor%20Object%20Reference) (OtherComp :type Primitive%20Component%20Object%20Reference) (OtherBodyIndex :type Integer) (bFromSweep :type Boolean) (SweepResult :type Hit%20Result%20Structure%20%28by%20ref%29))
  ;[0.09468 0 1 1 90] Leafs collision setup
  (CallFunction|Leaf 44 "leaf_44" 4e+01)
  (Utilities|FlowControl|DoOnce false
    (:Completed
      (CallFunction|SpawnNiagara (Transformation|GetWorldTransform (Variables|Default|GetLeaf_44))))))

(event OnComponentBeginOverlap(Leaf_45)
  (params (OverlappedComponent :type Primitive%20Component%20Object%20Reference) (OtherActor :type Actor%20Object%20Reference) (OtherComp :type Primitive%20Component%20Object%20Reference) (OtherBodyIndex :type Integer) (bFromSweep :type Boolean) (SweepResult :type Hit%20Result%20Structure%20%28by%20ref%29))
  ;[0.09468 0 1 1 90] Leafs collision setup
  (CallFunction|Leaf 45 "leaf_45" 4e+01)
  (Utilities|FlowControl|DoOnce false
    (:Completed
      (CallFunction|SpawnNiagara (Transformation|GetWorldTransform (Variables|Default|GetLeaf_45))))))

(event OnComponentBeginOverlap(Leaf_46)
  (params (OverlappedComponent :type Primitive%20Component%20Object%20Reference) (OtherActor :type Actor%20Object%20Reference) (OtherComp :type Primitive%20Component%20Object%20Reference) (OtherBodyIndex :type Integer) (bFromSweep :type Boolean) (SweepResult :type Hit%20Result%20Structure%20%28by%20ref%29))
  ;[0.09468 0 1 1 90] Leafs collision setup
  (CallFunction|Leaf 46 "leaf_46" 4e+01)
  (Utilities|FlowControl|DoOnce false
    (:Completed
      (CallFunction|SpawnNiagara (Transformation|GetWorldTransform (Variables|Default|GetLeaf_46))))))

(event OnComponentBeginOverlap(Leaf_47)
  (params (OverlappedComponent :type Primitive%20Component%20Object%20Reference) (OtherActor :type Actor%20Object%20Reference) (OtherComp :type Primitive%20Component%20Object%20Reference) (OtherBodyIndex :type Integer) (bFromSweep :type Boolean) (SweepResult :type Hit%20Result%20Structure%20%28by%20ref%29))
  ;[0.09468 0 1 1 90] Leafs collision setup
  (CallFunction|Leaf 47 "leaf_47" 4e+01)
  (Utilities|FlowControl|DoOnce false
    (:Completed
      (CallFunction|SpawnNiagara (Transformation|GetWorldTransform (Variables|Default|GetLeaf_47))))))

(event OnComponentBeginOverlap(Leaf_48)
  (params (OverlappedComponent :type Primitive%20Component%20Object%20Reference) (OtherActor :type Actor%20Object%20Reference) (OtherComp :type Primitive%20Component%20Object%20Reference) (OtherBodyIndex :type Integer) (bFromSweep :type Boolean) (SweepResult :type Hit%20Result%20Structure%20%28by%20ref%29))
  ;[0.09468 0 1 1 90] Leafs collision setup
  (CallFunction|Leaf 48 "leaf_48" 4e+01))

(event OnComponentBeginOverlap(Leaf_06)
  (params (OverlappedComponent :type Primitive%20Component%20Object%20Reference) (OtherActor :type Actor%20Object%20Reference) (OtherComp :type Primitive%20Component%20Object%20Reference) (OtherBodyIndex :type Integer) (bFromSweep :type Boolean) (SweepResult :type Hit%20Result%20Structure%20%28by%20ref%29))
  ;[0.09468 0 1 1 90] Leafs collision setup
  (CallFunction|Leaf 6 "leaf_06" 4e+01)
  (Utilities|FlowControl|DoOnce false
    (:Completed
      (CallFunction|SpawnNiagara (Transformation|GetWorldTransform (Variables|Default|GetLeaf_06))))))

(event OnComponentBeginOverlap(Leaf_07)
  (params (OverlappedComponent :type Primitive%20Component%20Object%20Reference) (OtherActor :type Actor%20Object%20Reference) (OtherComp :type Primitive%20Component%20Object%20Reference) (OtherBodyIndex :type Integer) (bFromSweep :type Boolean) (SweepResult :type Hit%20Result%20Structure%20%28by%20ref%29))
  ;[0.09468 0 1 1 90] Leafs collision setup
  (CallFunction|Leaf 7 "leaf_07" 4e+01)
  (Utilities|FlowControl|DoOnce false
    (:Completed
      (CallFunction|SpawnNiagara (Transformation|GetWorldTransform (Variables|Default|GetLeaf_07))))))

(event OnComponentBeginOverlap(Leaf_08)
  (params (OverlappedComponent :type Primitive%20Component%20Object%20Reference) (OtherActor :type Actor%20Object%20Reference) (OtherComp :type Primitive%20Component%20Object%20Reference) (OtherBodyIndex :type Integer) (bFromSweep :type Boolean) (SweepResult :type Hit%20Result%20Structure%20%28by%20ref%29))
  ;[0.09468 0 1 1 90] Leafs collision setup
  (CallFunction|Leaf 8 "leaf_08" 4e+01)
  (Utilities|FlowControl|DoOnce false
    (:Completed
      (CallFunction|SpawnNiagara (Transformation|GetWorldTransform (Variables|Default|GetLeaf_08))))))

(event OnComponentBeginOverlap(Leaf_09)
  (params (OverlappedComponent :type Primitive%20Component%20Object%20Reference) (OtherActor :type Actor%20Object%20Reference) (OtherComp :type Primitive%20Component%20Object%20Reference) (OtherBodyIndex :type Integer) (bFromSweep :type Boolean) (SweepResult :type Hit%20Result%20Structure%20%28by%20ref%29))
  ;[0.09468 0 1 1 90] Leafs collision setup
  (CallFunction|Leaf 9 "leaf_09" 4e+01)
  (Utilities|FlowControl|DoOnce false
    (:Completed
      (CallFunction|SpawnNiagara (Transformation|GetWorldTransform (Variables|Default|GetLeaf_09))))))

(event OnComponentBeginOverlap(Leaf_10)
  (params (OverlappedComponent :type Primitive%20Component%20Object%20Reference) (OtherActor :type Actor%20Object%20Reference) (OtherComp :type Primitive%20Component%20Object%20Reference) (OtherBodyIndex :type Integer) (bFromSweep :type Boolean) (SweepResult :type Hit%20Result%20Structure%20%28by%20ref%29))
  ;[0.09468 0 1 1 90] Leafs collision setup
  (CallFunction|Leaf 10 "leaf_10" 4e+01)
  (Utilities|FlowControl|DoOnce false
    (:Completed
      (CallFunction|SpawnNiagara (Transformation|GetWorldTransform (Variables|Default|GetLeaf_10))))))

(event Custom|Spawn_Niagara
  (params (Transform :type Transform))
  (bind (_location _rotation) (Math|Transform|BreakTransform Transform))
  ;[1 1 1 1 90] Spawn Niagara
  (Niagara|SpawnSystematLocation "/Game/Snow_FX/Niagara_particles/Fall_Snow_Emitter_System.Fall_Snow_Emitter_System" _location _rotation))

(event Custom|leaf
  (params (LeafId :type Integer) (leafname :type Name :default "leaf_00") (Move :type Float%20%28single-precision%29))
  ;[1 1 1 1 90] Send to Material
  (Utilities|HitLeaf LeafId leafname Move))

(fn ConstructionScript)