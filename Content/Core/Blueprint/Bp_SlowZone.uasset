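; Trigger zone actor that steadily shrinks the player's snowball while it is inside the box.
; Box begin and end overlaps with Bp_SnowBall toggle a Condition flag.
; While the flag is set, Tick subtracts a fixed step from the player pawn's Sphere world scale, with no delta-time scaling or minimum size.
; Despite the SlowZone name, nothing here changes speed directly.
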(event OnComponentBeginOverlap(Box)
  (params (OverlappedComponent :type Primitive%20Component%20Object%20Reference) (OtherActor :type Actor%20Object%20Reference) (OtherComp :type Primitive%20Component%20Object%20Reference) (OtherBodyIndex :type Integer) (bFromSweep :type Boolean) (SweepResult :type Hit%20Result%20Structure%20%28by%20ref%29))
  (Utilities|Casting|CastToBp_SnowBall OtherActor)
  (Variables|Default|SetCondition true))

(event OnComponentEndOverlap(Box)
  (params (OverlappedComponent :type Primitive%20Component%20Object%20Reference) (OtherActor :type Actor%20Object%20Reference) (OtherComp :type Primitive%20Component%20Object%20Reference) (OtherBodyIndex :type Integer))
  (Utilities|Casting|CastToBp_SnowBall OtherActor)
  (Variables|Default|SetCondition false))

(event EventTick
  (params (DeltaSeconds :type Float%20%28single-precision%29))
  (if (Variables|Default|GetCondition)
    (bind _asbp_snow_ball (Utilities|Casting|CastToBp_SnowBall (Game|Player|GetPlayerPawn 0)))
    (Transformation|SetWorldScale3D (Variables|/Game/Core/Blueprint/Bp_SnowBall.Bp_SnowBall_C|GetSphere _asbp_snow_ball) (- (Transformation|GetWorldScale (Variables|/Game/Core/Blueprint/Bp_SnowBall.Bp_SnowBall_C|GetSphere _asbp_snow_ball)) 0.01))))

(fn ConstructionScript)