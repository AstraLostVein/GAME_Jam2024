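; BP_Traps is an obstacle for the snowball, with a random mesh and a random scale on each axis set at BeginPlay.
; When its sphere overlaps a Bp_SnowBall, it checks the snowball sphere's Y world scale against a size threshold.
; A snowball at or above the threshold destroys the trap, while a smaller one shrinks by a fixed amount and leaves the trap in place.
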(event OnComponentBeginOverlap(Sphere)
  (params (OverlappedComponent :type Primitive%20Component%20Object%20Reference) (OtherActor :type Actor%20Object%20Reference) (OtherComp :type Primitive%20Component%20Object%20Reference) (OtherBodyIndex :type Integer) (bFromSweep :type Boolean) (SweepResult :type Hit%20Result%20Structure%20%28by%20ref%29))
  (bind _asbp_snow_ball (Utilities|Casting|CastToBp_SnowBall OtherActor))
  (if (>= (.y (Transformation|GetWorldScale (Variables|/Game/Core/Blueprint/Bp_SnowBall.Bp_SnowBall_C|GetSphere _asbp_snow_ball))) 2e+01)
    (Actor|DestroyActor)
    (else
      (Transformation|SetWorldScale3D (Variables|/Game/Core/Blueprint/Bp_SnowBall.Bp_SnowBall_C|GetSphere _asbp_snow_ball) (- (Transformation|GetWorldScale (Variables|/Game/Core/Blueprint/Bp_SnowBall.Bp_SnowBall_C|GetSphere _asbp_snow_ball)) "5.000000,5.000000,5.000000")))))

(event EventBeginPlay
  (bind _trap (Variables|Default|GetTrap))
  (bind _minscale (Variables|Default|GetMinScale))
  (bind _maxscale (Variables|Default|GetMaxScale))
  (bind _returnvalue (Math|Random|RandomFloatinRange _minscale _maxscale))
  (Transformation|SetWorldScale3D _trap (Math|Vector|MakeVector _returnvalue _returnvalue _returnvalue))
  (Components|StaticMesh|SetStaticMesh _trap (.OutItem (Utilities|Array|Random (Variables|Default|GetRandomMeshArray)))))

(fn ConstructionScript)