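; BP_TrapsTiny is a small trap that reacts when the player's snowball (Bp_SnowBall) rolls into it.
; BeginPlay gives the trap a random mesh and a random scale on each axis.
; On sphere overlap it prints a debug string, shakes the camera and compares the snowball's Y scale to a threshold.
; Large enough snowballs pass unharmed, smaller ones shrink by a set amount, and the trap is destroyed either way.
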(event OnComponentBeginOverlap(Sphere)
  (params (OverlappedComponent :type Primitive%20Component%20Object%20Reference) (OtherActor :type Actor%20Object%20Reference) (OtherComp :type Primitive%20Component%20Object%20Reference) (OtherBodyIndex :type Integer) (bFromSweep :type Boolean) (SweepResult :type Hit%20Result%20Structure%20%28by%20ref%29))
  (bind _asbp_snow_ball (Utilities|Casting|CastToBp_SnowBall OtherActor))
  (Development|PrintString "Hello")
  (Class|LegacyCameraShake|StartLegacyCameraShake (Game|GetPlayerCameraManager 0) "/Game/Core/Blueprint/Shake/CS_Hit.CS_Hit_C" 1.0 "CameraLocal" "0, 0, 0")
  (if (>= (.y (Transformation|GetWorldScale (Variables|/Game/Core/Blueprint/Bp_SnowBall.Bp_SnowBall_C|GetSphere _asbp_snow_ball))) (Variables|Default|GetHowBigYouNeedToBe?))
    (Collision|SetCollisionEnabled (Variables|Default|GetTrap) "NoCollision")
    (Actor|DestroyActor)
    (else
      (Transformation|SetWorldScale3D (Variables|/Game/Core/Blueprint/Bp_SnowBall.Bp_SnowBall_C|GetSphere _asbp_snow_ball) (- (Transformation|GetWorldScale (Variables|/Game/Core/Blueprint/Bp_SnowBall.Bp_SnowBall_C|GetSphere _asbp_snow_ball)) (Variables|Default|GetHowMuchYouLose)))
      (Actor|DestroyActor))))

(event EventBeginPlay
  (bind _trap (Variables|Default|GetTrap))
  (bind _minscale (Variables|Default|GetMinScale))
  (bind _maxscale (Variables|Default|GetMaxScale))
  (bind _returnvalue (Math|Random|RandomFloatinRange _minscale _maxscale))
  (Transformation|SetWorldScale3D _trap (Math|Vector|MakeVector _returnvalue _returnvalue _returnvalue))
  (Components|StaticMesh|SetStaticMesh _trap (.OutItem (Utilities|Array|Random (Variables|Default|GetRandomMeshArray)))))

(fn ConstructionScript)