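; Level-end trigger actor that runs the finish sequence when the Bp_SnowBall overlaps its box.
; A DoOnce gate lets the sequence run once, blending player 0's view to this actor.
; After a short delay it applies a single forward force to the snowball's sphere along its arrow, then shows WBP_FinalScore with the snowball passed as PlayerRef.
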(event OnComponentBeginOverlap(Box)
  (params (OverlappedComponent :type Primitive%20Component%20Object%20Reference) (OtherActor :type Actor%20Object%20Reference) (OtherComp :type Primitive%20Component%20Object%20Reference) (OtherBodyIndex :type Integer) (bFromSweep :type Boolean) (SweepResult :type Hit%20Result%20Structure%20%28by%20ref%29))
  (bind _asbp_snow_ball (Utilities|Casting|CastToBp_SnowBall OtherActor))
  (Utilities|FlowControl|DoOnce false
    (:Completed
      (Game|Player|SetViewTargetwithBlend (Game|GetPlayerController 0) self 1.5 "VTBlend_Linear" 0.0 false)
      (Utilities|FlowControl|Delay 2.0)
      (Physics|AddForce (Variables|/Game/Core/Blueprint/Bp_SnowBall.Bp_SnowBall_C|GetSphere _asbp_snow_ball) (* (Math|Vector|GetForwardVector (Variables|/Game/Core/Blueprint/Bp_SnowBall.Bp_SnowBall_C|GetArrow _asbp_snow_ball)) 2.5e+03) "None" false)
      (bind _returnvalue (UserInterface|CreateWidget "/Game/Core/Widget/WBP_FinalScore.WBP_FinalScore_C" 0 _asbp_snow_ball))
      (UserInterface|Viewport|AddtoViewport _returnvalue 0))))

(fn ConstructionScript)